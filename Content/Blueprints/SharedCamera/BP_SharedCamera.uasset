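; Shared camera actor that keeps the players in view with a single zooming spring-arm camera.
; Each tick it moves to the average location of all player pawns.
; The farthest pawn's distance from that center maps through a clamped range to a zoom factor that scales the spring arm length.
; MakePlayerReference stores up to two character references, which the camera logic here does not use.
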(event Custom|MakePlayerReference
  (params (CharacterRef :type BP%20Player%20Character%20Object%20Reference))
  (Variables|PlayerRef|GetPlayerOne
    (:then
      (Variables|PlayerRef|SetPlayerTwo CharacterRef))
    (:else
      (Variables|PlayerRef|SetPlayerOne CharacterRef))))

(event EventBeginPlay)

(event Collision|EventActorBeginOverlap
  (params (OtherActor :type Actor%20Object%20Reference)))

(event EventTick
  (params (DeltaSeconds :type Float%20%28single-precision%29))
  ;[0.15 0.15 0.15 0.5] Set Camera Location
  (bind _returnvalue (Class|GameModeBase|GetNumPlayers (Game|GetGameMode)))
  (Variables|CameraDistances|SetLocationSum "0, 0, 0")
  (for _index (range 0 (- _returnvalue 1))
    (Variables|CameraDistances|SetLocationSum (+ (Variables|CameraDistances|GetLocationSum) (Transformation|GetActorLocation (Game|Player|GetPlayerPawn _index)))))
  (Transformation|SetActorLocation (/ (Variables|CameraDistances|GetLocationSum) _returnvalue) false false)
  ;[0.15 0.15 0.15 0.5] CameraBetweenCharacters
  (Variables|CameraDistances|SetBiggestDistanceFromCenter 0.0)
  (bind _returnvalue_2 (Class|GameModeBase|GetNumPlayers (Game|GetGameMode)))
  (for _index_2 (range 0 (- _returnvalue_2 1))
    (if (> (Math|Vector|Distance(Vector) (Transformation|GetActorLocation) (Transformation|GetActorLocation (Game|Player|GetPlayerPawn _index_2))) (Variables|CameraDistances|GetBiggestDistanceFromCenter))
      (Variables|CameraDistances|SetBiggestDistanceFromCenter (Math|Vector|Distance(Vector) (Transformation|GetActorLocation) (Transformation|GetActorLocation (Game|Player|GetPlayerPawn _index_2))))))
  (Variables|/Script/Engine.SpringArmComponent|SetTargetArmLength (Variables|Default|GetSpringArm) (* (Math|Float|MapRangeClamped (Variables|CameraDistances|GetBiggestDistanceFromCenter) (Variables|CameraDistances|GetMinDistanceFromCenter) (Variables|CameraDistances|GetMaxDistanceFromCenter) (Variables|CameraDistances|GetMinZoom) (Variables|CameraDistances|GetMaxZoom)) (Variables|CameraDistances|GetMinArmLengthValue))))

(fn ConstructionScript)