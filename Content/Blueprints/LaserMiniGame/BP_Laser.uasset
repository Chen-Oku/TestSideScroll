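; BP_Laser is a laser beam actor for the laser mini-game that shortens when something blocks it.
; Each Tick it line-traces on the Visibility channel along the Arrow's forward vector, up to LaserLength.
; The hit distance, or LaserLength when unblocked, becomes MeshLength, which drives the LaserCylinder's X scale.
; The trace leaves persistent debug lines, and the actor applies no effect to what it hits.
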(event EventBeginPlay)

(event Collision|EventActorBeginOverlap
  (params (OtherActor :type Actor%20Object%20Reference)))

(event EventTick
  (params (DeltaSeconds :type Float%20%28single-precision%29))
  (bind _arrow (Variables|Default|GetArrow))
  (bind _returnvalue (Transformation|GetWorldLocation _arrow))
  (bind _outhit (Collision|LineTraceByChannel _returnvalue (+ _returnvalue (* (Math|Vector|GetForwardVector _arrow) (Variables|Default|GetLaserLength))) "TraceTypeQuery1" false 0 "Persistent"))
  (if (.bBlockingHit (Collision|BreakHitResult _outhit))
    (bind _output_get (Variables|Default|SetMeshLength (.Distance (Collision|BreakHitResult _outhit))))
    (Transformation|SetWorldScale3D (Variables|Default|GetLaserCylinder) (Math|Vector|MakeVector (/ _output_get 1e+01) 2e+01 2e+01))
    (else
      (bind _output_get_2 (Variables|Default|SetMeshLength (Variables|Default|GetLaserLength)))
      (Transformation|SetWorldScale3D (Variables|Default|GetLaserCylinder) (Math|Vector|MakeVector (/ _output_get_2 1e+01) 2e+01 2e+01)))))

(fn ConstructionScript)