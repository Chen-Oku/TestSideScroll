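; Health component that tracks current health against a maximum and flags death.
; BeginPlay calls Health to fill CurrentHealth to MaxHealth.
; ReciveDamage resets health to MaxHealth before subtracting a fixed amount with clamping, so hits do not accumulate.
; It sets IsDead when the result reaches zero, and Tick is unused.
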(event EventBeginPlay
  (CallFunction|Health))

(event EventTick
  (params (DeltaSeconds :type Float%20%28single-precision%29)))

(fn Health
  (Variables|Default|SetCurrentHealth (Variables|Default|GetMaxHealth)))

(fn ReciveDamage
  (bind _output_get (Variables|Default|SetCurrentHealth (Variables|Default|GetMaxHealth)))
  (Variables|Default|SetCurrentHealth (Math|Integer|Clamp(Integer) (- _output_get 10) 0 (Variables|Default|GetMaxHealth)))
  (if (<= (Variables|Default|GetCurrentHealth) 0)
    (Variables|Default|SetIsDead true)))